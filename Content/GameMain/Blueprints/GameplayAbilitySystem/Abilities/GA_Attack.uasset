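; GA_Attack is the player's attack Gameplay Ability, playing M_Attack from the montage section name stored on BP_Player.
; It ends itself when a Player.Status.CombowindowOpen gameplay event arrives, while the montage is set to keep playing after the ability ends.
; Disconnected leftover nodes hold an alternative combo approach using a CanCombo tag check, loose tags and a window-closed event.
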(event `self.K2_ActivateAbility`
  (bind _asbp_player (cast `/Game/GameMain/Blueprints/Character/Player/BP_Player` (`self.GetAvatarActorFromActorInfo`)))
  (`AbilityTask_PlayMontageAndWait.CreatePlayMontageAndWaitProxy` "None" "/Game/GameMain/Blueprints/Character/Player/Montages/M_Attack.M_Attack" 1.0 (`/Game/GameMain/Blueprints/Character/Player/BP_Player.MontageSectionName` _asbp_player) false
    (:`then`
      (`AbilityTask_WaitGameplayEvent.WaitGameplayEvent` (struct :`TagName` "Player.Status.CombowindowOpen") null
        (:`EventReceived`
          (`self.K2_EndAbility`))))))