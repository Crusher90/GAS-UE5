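; AI controller Blueprint for a close-ranged enemy, with its event graph logic currently disconnected.
; BeginPlay and the perception updated and forgotten events are all empty.
; Unwired nodes would run the default behavior tree, set TargetActor and IsAgro for actors implementing GPlayerInterface, and clear both and restart logic when a target is forgotten.
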(event `self.ReceiveBeginPlay`)

(event `self.PerceptionComp.OnTargetPerceptionUpdated`
  (params (Actor :type "Actor Object Reference") (Stimulus :type "AIStimulus Structure")))

(event `self.PerceptionComp.OnTargetPerceptionForgotten`
  (params (Actor :type "Actor Object Reference")))

(fn `UserConstructionScript`)